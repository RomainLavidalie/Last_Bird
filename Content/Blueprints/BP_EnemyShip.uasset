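; Enemy ship Blueprint that tracks a Health value and destroys the actor when it drops to zero or below.
; AffectHealth passes a signed delta to UpdateHealth, which adds it to Health and refreshes IsDead through UpdateIsDead, then destroys the actor if dead.
; Tick independently repeats the zero-health check every frame, and both Tick and AffectHealth print Health for debugging.
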(event `self.ReceiveTick`
  (params (DeltaSeconds :type "Float (single-precision)"))
  (bind _health (`self.Health`))
  (`|ExecutionSequence`
    (:`then_0`
      (`KismetSystemLibrary.PrintString` (`KismetStringLibrary.Conv_IntToString` _health)))
    (:`then_1`
      (if (<= _health 0)
        (`self.K2_DestroyActor`)))))

(event `/Game/Blueprints/BPI_Damageable.AffectHealth`
  (params (Delta :type Integer))
  (bind _new_health (`self.UpdateHealth` Delta))
  (`KismetSystemLibrary.PrintString` (`KismetStringLibrary.Conv_IntToString` _new_health))
  (if (`self.IsDead`)
    (`self.K2_DestroyActor`)))

(event `UpdateIsDead`
  (if (<= (`self.Health`) 0)
    (set `self.IsDead` true)
    (else
      (set `self.IsDead` false))))

(fn `UpdateHealth`
  (params (Delta :type Integer))
  (returns (`New Health` :type Integer))
  (bind _output_get (set `self.Health` (+ Delta (`self.Health`))))
  (`self.UpdateIsDead`)
  (return _output_get))

(fn `UserConstructionScript`)