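; Player-controlled ship that moves on input axes, turns to face the mouse cursor and fires twin lasers.
; Tick sets its yaw toward the cursor's Visibility trace hit, keeping pitch and roll at zero.
; Holding Shoot fires BP_Laser from two arrow components immediately, then on a looping timer driven by ShotsPerSecond.
; A DoOnce guards firing until release clears the timer and resets it.
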(event `Fire Projectile`
  ;[1 1 1] Shooting
  (`|SpawnActorFromClass` "/Game/Blueprints/BP_Laser.BP_Laser_C" (`SceneComponent.K2_GetComponentToWorld` (`self.ArrowL`)) "Undefined" "OverrideRootScale" null null)
  (`|SpawnActorFromClass` "/Game/Blueprints/BP_Laser.BP_Laser_C" (`SceneComponent.K2_GetComponentToWorld` (`self.ArrowR`)) "Undefined" "OverrideRootScale" null null))

(event `InputAction|Shoot`
  (params (Key :type "Key Structure"))
  (:`Pressed`
    (`self.Start Firing`))
  (:`Released`
    (`self.Stop Firing`)))

(event `Start Firing`
  (`/Engine/EditorBlueprintResources/StandardMacros.DoOnce` false :!label _label
    (:`Completed`
      (`self.Fire Projectile`)
      (`KismetSystemLibrary.K2_SetTimer` null "Fire Projectile" (/ 1.0 (`self.Shots per Second`)) true))))

(event `self.ReceiveTick`
  (params (DeltaSeconds :type "Float (single-precision)"))
  (`self.K2_SetActorRotation` (`KismetMathLibrary.MakeRotator` 0.0 0.0 (.yaw (`KismetMathLibrary.FindLookAtRotation` (`self.K2_GetActorLocation`) (`.Location` (`GameplayStatics.BreakHitResult` (`PlayerController.GetHitResultUnderCursorByChannel` (`GameplayStatics.GetPlayerController` 0) "TraceTypeQuery1" true))))))))

(event `Stop Firing`
  (`KismetSystemLibrary.K2_ClearTimer` null "Fire Projectile")
  (goto _label :!via `Reset`))

(event `InputAxis|UpDown`
  (params (AxisValue :type "Float (single-precision)"))
  (`self.MoveForward` AxisValue))

(event `InputAxis|LeftRight`
  (params (AxisValue :type "Float (single-precision)"))
  (`self.AddMovementInput` (0.0 -1.0 0.0) AxisValue))

(fn `UserConstructionScript`)